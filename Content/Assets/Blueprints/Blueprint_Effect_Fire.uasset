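; Fire effect Blueprint that grows a fire particle effect and plays its sounds when triggered.
; BeginPlay silences the fire and explosion audio components.
; ToggleVisible plays the FireGrowth timeline, which drives the uniform relative scale of PFire.
; Event tracks on that timeline start the explosion cue and the fire audio.
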(event Custom|ToggleVisible
  (bind _fire_growth (Timeline|FireGrowth Play)
    (:Update
      (Transformation|SetRelativeScale3D (Variables|Default|GetP_Fire) (Math|Vector|MakeVector _fire_growth _fire_growth _fire_growth)))
    (:Explosion
      (Audio|Components|Audio|Play (Variables|Audio|GetExplosion_Cue) 0.0))
    (:Fire
      (Audio|Components|Audio|Play (Variables|Audio|GetFire%20Audio) 0.0))))

(event EventBeginPlay
  (Audio|Components|Audio|Stop (Variables|Audio|GetFire%20Audio))
  (Audio|Components|Audio|Stop (Variables|Audio|GetExplosion_Cue)))

(fn ConstructionScript)