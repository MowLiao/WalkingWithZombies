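; House Blueprint for the scenic landscape level that drives a configurable, optionally flickering point light.
; The construction script applies the Brightness, Color and SourceRadius variables to the light.
; On BeginPlay, a looping random delay of up to five seconds toggles the light's visibility while LightFlicker is true.
; With LightFlicker false, the light turns off after the first delay and stays hidden.
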(event EventBeginPlay
  (bind _pointlight (Variables|Default|GetPointLight))
  ;[1 1 1] Toggles the light to flicker on and off
  (Utilities|FlowControl|Delay (* (Math|Random|RandomFloat) 5.0) :!label _label)
  (Rendering|ToggleVisibility _pointlight false)
  (if (Variables|Default|GetLightFlicker)
    (goto _label)
    (else
      (Rendering|SetVisibility _pointlight false false))))

(event Collision|EventActorBeginOverlap
  (params (OtherActor :type Actor%20Object%20Reference)))

(event EventTick
  (params (DeltaSeconds :type Float%20%28single-precision%29)))

(fn ConstructionScript
  (bind _pointlight (Variables|Default|GetPointLight))
  ;[1 1 1] Constructs light with source
  (Rendering|Components|Light|SetIntensity _pointlight (Variables|Default|GetBrightness))
  (Rendering|Components|Light|SetLightColor _pointlight (Variables|Default|GetColor) true)
  (Class|PointLightComponent|SetSourceRadius _pointlight (Variables|Default|GetSource%20Radius)))