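; Zombie character Blueprint that provides keyboard and mouse controls for when a player possesses it.
; BeginPlay calls EnableInput, and the forward, back and strafe axes feed AddMovementInput along directions built from control rotation yaw alone.
; The mouse X axis turns the controller yaw; there is no pitch control.
; Tick, overlap, possession event and construction script are empty.
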(event EventBeginPlay
  (Input|EnableInput 0))

(event Collision|EventActorBeginOverlap
  (params (OtherActor :type Actor%20Object%20Reference)))

(event EventPossessed
  (params (NewController :type Controller%20Object%20Reference)))

(event EventTick
  (params (DeltaSeconds :type Float%20%28single-precision%29)))

(event Input|AxisEvents|InputAxismousex
  (params (AxisValue :type Float%20%28single-precision%29))
  ;[1 1 1] Possession Controls
  ;;[1 1 1] Camera Control
  (Pawn|Input|AddControllerYawInput AxisValue))

(event Input|AxisEvents|InputAxisForward
  (params (AxisValue :type Float%20%28single-precision%29))
  ;[1 1 1] Possession Controls
  ;;[1 1 1] Keyboard
  (Pawn|Input|AddMovementInput (Math|Vector|GetForwardVector (Math|Rotator|MakeRotator 0.0 0.0 (.Yaw (Math|Rotator|BreakRotator (Pawn|GetControlRotation :!class /Script/Engine.Pawn))))) AxisValue false))

(event Input|AxisEvents|InputAxisStrafe_Right
  (params (AxisValue :type Float%20%28single-precision%29))
  ;[1 1 1] Possession Controls
  ;;[1 1 1] Keyboard
  (Pawn|Input|AddMovementInput (Math|Vector|GetRightVector (Math|Rotator|MakeRotator 0.0 0.0 (.Yaw (Math|Rotator|BreakRotator (Pawn|GetControlRotation :!class /Script/Engine.Pawn))))) AxisValue false))

(event Input|AxisEvents|InputAxisBack
  (params (AxisValue :type Float%20%28single-precision%29))
  ;[1 1 1] Possession Controls
  ;;[1 1 1] Keyboard
  (Pawn|Input|AddMovementInput (Math|Vector|GetForwardVector (Math|Rotator|MakeRotator 0.0 0.0 (.Yaw (Math|Rotator|BreakRotator (Pawn|GetControlRotation :!class /Script/Engine.Pawn))))) AxisValue false))

(event Input|AxisEvents|InputAxisStrafe_Left
  (params (AxisValue :type Float%20%28single-precision%29))
  ;[1 1 1] Possession Controls
  ;;[1 1 1] Keyboard
  (Pawn|Input|AddMovementInput (Math|Vector|GetRightVector (Math|Rotator|MakeRotator 0.0 0.0 (.Yaw (Math|Rotator|BreakRotator (Pawn|GetControlRotation :!class /Script/Engine.Pawn))))) AxisValue false))

(fn ConstructionScript)