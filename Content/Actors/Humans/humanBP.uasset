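; Human character Blueprint for a scripted actor that walks to a target and can be registered with the zombie crowd AI.
; SetHumanInBT and ClearHumanInBT set or unset the human on every CrowdAI_Con controller for the zombie behavior tree.
; MoveToTarget uses AI Move To and, shortly after arrival, destroys the human.
; The final human first clears the crowd reference and fires FullHouse on the ScenicEvents actor found at BeginPlay.
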(event Custom|MoveToTarget
  (params (MoveToLocation :type Target%20Point%20Object%20Reference))
  (bind _self self)
  ;[1 1 1] Move human to target
  (bind _output_get (Variables|Default|SetthisAICon (AI|GetAIController _self)))
  (AI|AIMoveTo _output_get _self (Transformation|GetActorLocation MoveToLocation) 0 5.0 false
    (:OnSuccess
      (Utilities|FlowControl|Delay 1.5)
      (if (Variables|Default|GetFinalHuman)
        (CallFunction|ClearHumaninBT)
        (Default|FullHouse (Variables|Default|GetscenicEventsBP)))
      (Actor|DestroyActor))))

(event Custom|SetHumanInBT
  ;[1 1 1] Refer to self in zombie behaviour tree
  (bind _outactors (Actor|GetAllActorsOfClass "/Game/Actors/Crowd/crowdAI_Con.crowdAI_Con_C"))
  (for _array_element _outactors
    (Default|SetHuman _array_element self)))

(event Custom|ClearHumanInBT
  ;[1 1 1] Reset human value in zombie behaviour tree
  (bind _outactors (Actor|GetAllActorsOfClass "/Game/Actors/Crowd/crowdAI_Con.crowdAI_Con_C"))
  (for _array_element _outactors
    (Default|UnsetHuman _array_element)))

(event EventBeginPlay
  ;[1 1 1] Get the events BP
  (bind _outactors (Actor|GetAllActorsOfClass "/Game/Levels/scenicEvents.scenicEvents_C"))
  (for _array_element _outactors
    _)
  (Variables|Default|SetscenicEventsBP _array_element))

(event Collision|EventActorBeginOverlap
  (params (OtherActor :type Actor%20Object%20Reference)))

(event EventTick
  (params (DeltaSeconds :type Float%20%28single-precision%29)))

(fn ConstructionScript)