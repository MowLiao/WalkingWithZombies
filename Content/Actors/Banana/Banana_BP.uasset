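; Banana_BP is an actor for a banana that bobs and spins in place and disappears when touched.
; Each Tick advances a float counter and adds a sine-driven vertical offset and a yaw increment to the StaticMesh, with sweep on the move.
; Any overlap with the StaticMesh destroys the actor, with no filter on the overlapping actor and no other effect.
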(event OnComponentBeginOverlap(StaticMesh)
  (params (OverlappedComponent :type Primitive%20Component%20Object%20Reference) (OtherActor :type Actor%20Object%20Reference) (OtherComp :type Primitive%20Component%20Object%20Reference) (OtherBodyIndex :type Integer) (bFromSweep :type Boolean) (SweepResult :type Hit%20Result%20Structure%20%28by%20ref%29))
  ;[1 1 1] Disappear on Touch
  (Actor|DestroyActor))

(event EventBeginPlay)

(event Collision|EventActorBeginOverlap
  (params (OtherActor :type Actor%20Object%20Reference)))

(event EventTick
  (params (DeltaSeconds :type Float%20%28single-precision%29))
  ;[1 1 1] Float and rotate
  (bind _output_get (Variables|Default|Setfloat_tick (+ (Variables|Default|Getfloat_tick) (* 1.0 (Variables|Default|Getfloat_incr)))))
  (Transformation|AddRelativeLocation (Variables|Default|GetStaticMesh) (Math|Vector|MakeVector 0.0 0.0 (* (Math|Trig|Sin(Degrees) _output_get) (Variables|Default|Getfloat_mag))) true false)
  (Transformation|AddRelativeRotation (Variables|Default|GetStaticMesh) (Math|Rotator|MakeRotator 0.0 0.0 (Variables|Default|Getrot_incr)) false false))

(fn ConstructionScript)